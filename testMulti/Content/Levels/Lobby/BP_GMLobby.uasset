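; Lobby game mode that gathers joining players and sends the server to L_Game once the session is full.
; It tracks player controllers on login and logout, and each login restarts a short retriggerable delay before comparing player count with the session's connection limit.
; Excess players are kicked from the end of the list as "Serveur complet".
; A full lobby then updates the session and runs serverTravel after a pause.
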(event `self.K2_PostLogin`
  (params (NewPlayer :type "PlayerController Object Reference"))
  (`KismetArrayLibrary.Array_AddUnique` (`self.Player Controllers`) NewPlayer)
  (`KismetSystemLibrary.RetriggerableDelay` 2.0)
  (bind (_numconnections _numprivateconnections _bislan _bisdedicated _ballowinvites _ballowjoininprogress _bisanticheatenabled _builduniqueid _extrasettings) (`AdvancedSessionsLibrary.GetSessionSettings`)
    (:`OnSuccess`
      (if (> (`KismetArrayLibrary.Array_Length` (`GameStateBase.PlayerArray` (`GameplayStatics.GetGameState`))) _numconnections)
        (bind (_arrayindex _arrayelement) (`/Engine/EditorBlueprintResources/StandardMacros.ReverseForEachLoop` (`self.Player Controllers`))
          (:`LoopBody`
            (if (>= _arrayindex _numconnections)
              (`AdvancedSessionsLibrary.KickPlayer` _arrayelement "Serveur complet")))
          (:`Completed`
            (`UpdateSessionCallbackProxyAdvanced.UpdateSession` _extrasettings _numconnections :!label _label
              (:`OnSuccess`
                (`KismetSystemLibrary.Delay` 5.0)
                (`KismetSystemLibrary.ExecuteConsoleCommand` "serverTravel L_Game" null)))))
        (elif (== (`KismetArrayLibrary.Array_Length` (`GameStateBase.PlayerArray` (`GameplayStatics.GetGameState`))) _numconnections)
          (goto _label))))))

(event `self.K2_OnLogout`
  (params (ExitingController :type "Controller Object Reference"))
  (bind _asplayer_controller (cast `PlayerController` ExitingController))
  (`KismetArrayLibrary.Array_RemoveItem` (`self.Player Controllers`) _asplayer_controller))

(fn `UserConstructionScript`)