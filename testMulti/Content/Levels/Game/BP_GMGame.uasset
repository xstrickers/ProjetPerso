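; Game mode for a session-based multiplayer driving level that holds car spawning until the lobby is full.
; Each joining controller is tracked and the player count compared to the session's connection limit, kicking surplus players as "Serveur complet".
; At or above the limit, it updates the session, then spawns and possesses a BP_OffroadCar per controller at index-named player starts.
; Logout untracks controllers; an unconnected two-player spawn variant remains unused.
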(event `self.HandleStartingNewPlayer`
  (params (NewPlayer :type "PlayerController Object Reference"))
  ;[1 1 1] With Player check
  (`KismetArrayLibrary.Array_AddUnique` (`self.playerControllers`) NewPlayer)
  (bind (_numconnections _numprivateconnections _bislan _bisdedicated _ballowinvites _ballowjoininprogress _bisanticheatenabled _builduniqueid _extrasettings) (`AdvancedSessionsLibrary.GetSessionSettings`)
    (:`OnSuccess`
      (if (> (`KismetArrayLibrary.Array_Length` (`GameStateBase.PlayerArray` (`GameplayStatics.GetGameState`))) _numconnections)
        (bind (_arrayindex _arrayelement) (`/Engine/EditorBlueprintResources/StandardMacros.ReverseForEachLoop` (`self.playerControllers`))
          (:`LoopBody`
            (if (>= _arrayindex _numconnections)
              (`AdvancedSessionsLibrary.KickPlayer` _arrayelement "Serveur complet")))
          (:`Completed`
            (`UpdateSessionCallbackProxyAdvanced.UpdateSession` _extrasettings _numconnections :!label _label
              (:`OnSuccess`
                (for (_array_element _array_index) (`self.playerControllers`)
                  (bind _returnvalue (`|SpawnActorFromClass` "/Game/Bluprints/BP_OffroadCar.BP_OffroadCar_C" (`self.GetTransform` (`self.K2_FindPlayerStart` _array_element (`KismetStringLibrary.Conv_IntToString` _array_index))) "Undefined" "MultiplyWithRoot" null null))
                  (`Controller.Possess` _array_element _returnvalue))))))
        (elif (== (`KismetArrayLibrary.Array_Length` (`GameStateBase.PlayerArray` (`GameplayStatics.GetGameState`))) _numconnections)
          (goto _label))))))

(event `self.K2_OnLogout`
  (params (ExitingController :type "Controller Object Reference"))
  (bind _asplayer_controller (cast `PlayerController` ExitingController))
  (`KismetArrayLibrary.Array_RemoveItem` (`self.playerControllers`) _asplayer_controller))

(fn `UserConstructionScript`)