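; BP_Tracker is a race tracker for an offroad car, meant to manage checkpoints, laps and race setup.
; StartSequence numbers the checkpoints, activates the first and binds their cleared events to a handler that calls LapCheck and plays a sound.
; ApplySettings passes MaxLaps to the car and starts its game setup.
; BeginPlay is empty, the car-cast startup chain is unconnected, and the helper functions, including LapCheck, are stubs.
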(event `self.ReceiveBeginPlay`)

(event `ApplySettings`
  (bind _as_bp_offroad_car (`self.As BP Offroad Car`))
  (set `/Game/Bluprints/BP_OffroadCar.MaxLaps` (`self.MaxLaps`) _as_bp_offroad_car)
  (`self.UpdateTimes`)
  (`/Game/Bluprints/BP_OffroadCar.StartGameSetup` _as_bp_offroad_car))

(event `StartSequence`
  (bind _checkpoints (`self.Checkpoints`))
  (for (_array_element _array_index) (`self.Checkpoints`)
    (set `/Game/Bluprints/BP_Checkpoint.NextCheckpoint` (+ _array_index 1) _array_element)
    (set `self.TotalCheckpoints` (`KismetArrayLibrary.Array_Length` _checkpoints))
    (`self.ActivateCheckpoint` (`|GetArrayItem` _checkpoints))
    (for _array_element_2 (`self.Checkpoints`)
      (add `/Game/Bluprints/BP_Checkpoint.CheckpointCleared` _array_element_2 (delegate `CheckpointCleared_Event`)))))

(event `CheckpointCleared_Event`
  (params (NextCheckpoint :type Integer))
  (`self.LapCheck` NextCheckpoint)
  (`AudioComponent.Play` (`AmbientSound.AudioComponent` (`self.CheckpointSound`)) 0.0)
  (if (`/Game/Bluprints/BP_OffroadCar.RaceComplete` (`self.As BP Offroad Car`))
    _))

(fn `ActivateCheckpoint`
  (params (NextCheckpoint :type "/Game/Bluprints/BP_Checkpoint Object Reference")))

(fn `LapCheck`
  (params (Checkpoint :type Integer)))

(fn `RaceCompleteCheck`
  (returns (IsRaceComplete :type Boolean))
  (return false))

(fn `UpdateTimes`)

(fn `UserConstructionScript`)